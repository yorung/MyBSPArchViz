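; BP_LightSwitch is a switch Blueprint that turns a tagged group of Light actors on or off.
; SetTurnedOn acts only when the state changes, while Toggle flips it; both then call Apply.
; Apply finds every Light actor carrying TargetActorTag and sets its light component's visibility to match TurnedOn.
; Its event graph and construction script are empty, so nothing in the Blueprint itself triggers the switch.
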(fn `Apply`
  (bind _outactors (`GameplayStatics.GetAllActorsOfClassWithTag` "/Script/Engine.Light" (`self.TargetActorTag`)))
  (for _array_element _outactors
    (`SceneComponent.SetVisibility` (`Light.LightComponent` _array_element) (`self.bTurnedOn`) false)))

(fn `SetTurnedOn`
  (params (bInTurnedOn :type Boolean))
  (if (!= (stale _output_get) bInTurnedOn)
    (bind _output_get (set `self.bTurnedOn` (`local.bInTurnedOn`)))
    (`self.Apply`)
    (else
      (return))))

(fn `Toggle`
  (bind _output_get (set `self.bTurnedOn` (not (stale _output_get))))
  (`self.Apply`))

(fn `UserConstructionScript`)