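; BP_PanoramaSettings configures Stereo Panoramic capture for rendering 360-degree frames to a local folder.
; BeginPlay runs console commands that set rendering options and frame cap, then the SP capture parameters: output directory, slice size and angles, render passes, bit depth and monoscopic mode.
; Only the final color pass is enabled.
; Unconnected nodes hold commands for a 360 movie or single screenshot, so play alone triggers no capture.
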(event `self.ReceiveBeginPlay`
  ;[1 1 1] Rendering Commands
  (`KismetSystemLibrary.ExecuteConsoleCommand` "r.ToneMapperFilm 1" null)
  (`KismetSystemLibrary.ExecuteConsoleCommand` "r.AllowOcclusionQueries 0" null)
  (`KismetSystemLibrary.ExecuteConsoleCommand` "t.MaxFPS 60" null)
  ;[1 1 1] Capture Parameters
  (`KismetSystemLibrary.ExecuteConsoleCommand` "SP.OutputDir C:/PanoramicCaptureFrames" null)
  (`KismetSystemLibrary.ExecuteConsoleCommand` "SP.StepCaptureWidth 6144" null)
  (`KismetSystemLibrary.ExecuteConsoleCommand` "SP.CaptureSlicePixelWidth 720" null)
  (`KismetSystemLibrary.ExecuteConsoleCommand` "SP.HorizontalAngularIncrement 2" null)
  (`KismetSystemLibrary.ExecuteConsoleCommand` "SP.VerticalAngularIncrement 15" null)
  (`KismetSystemLibrary.ExecuteConsoleCommand` "SP.ConcurrentCaptures 8" null)
  (`KismetSystemLibrary.ExecuteConsoleCommand` "SP.CaptureHorizontalFOV 30" null)
  (`KismetSystemLibrary.ExecuteConsoleCommand` "SP.ShouldOverrideInitialYaw 0" null)
  ;[1 1 1] Render Passes
  (`KismetSystemLibrary.ExecuteConsoleCommand` "SP.OutputFinalColor 1" null)
  (`KismetSystemLibrary.ExecuteConsoleCommand` "SP.OutputSceneDepth 0" null)
  (`KismetSystemLibrary.ExecuteConsoleCommand` "SP.OutputWorldNormal 0" null)
  (`KismetSystemLibrary.ExecuteConsoleCommand` "SP.OutputBaseColor 0" null)
  (`KismetSystemLibrary.ExecuteConsoleCommand` "SP.OutputAmbientOcclusion 0" null)
  (`KismetSystemLibrary.ExecuteConsoleCommand` "SP.OutputRoughness 0" null)
  (`KismetSystemLibrary.ExecuteConsoleCommand` "SP.OutputMetalic 0" null)
  ;[1 1 1] Output Bitdepth
  (`KismetSystemLibrary.ExecuteConsoleCommand` "SP.OutputBitDepth 32" null)
  ;[1 1 1] Mono or Stereo mode
  (`KismetSystemLibrary.ExecuteConsoleCommand` "SP.Monoscopic true" null))

(fn `UserConstructionScript`)