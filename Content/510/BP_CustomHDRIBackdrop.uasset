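; BP_CustomHDRIBackdrop is an HDRI backdrop actor that displays a cubemap on a configurable mesh.
; Its construction script scales the mesh from its bounds to a size in meters, then creates a camera- or center-projection dynamic material.
; The material receives the cubemap, intensity, lighting distance, projection position and an angle from negated actor yaw.
; The scene component's rotation is flattened to yaw only.
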(fn `CreateMaterial`
  (bind _scenecomponent (`self.SceneComponent`))
  (bind (_returnvalue_roll _returnvalue_pitch _returnvalue_yaw) (`KismetMathLibrary.BreakRotator` (`SceneComponent.K2_GetComponentRotation` _scenecomponent)))
  (`|ExecutionSequence`
    (:`then_0`
      (if (`self.UseCameraProjection`)
        (bind _returnvalue (`KismetMaterialLibrary.CreateDynamicMaterialInstance` "/HDRIBackdrop/Materials/MI_HDRI_CameraProjection.MI_HDRI_CameraProjection" "HDRI_MID"))
        (bind _output_get (set `self.MaterialInstance` _returnvalue))
        (else
          (bind _returnvalue_2 (`KismetMaterialLibrary.CreateDynamicMaterialInstance` "/HDRIBackdrop/Materials/MI_HDRI_CenterProjection.MI_HDRI_CenterProjection" "HDRI_MID"))
          (bind _output_get_2 (set `self.MaterialInstance` _returnvalue_2))))
      (`MaterialInstanceDynamic.SetTextureParameterValue` _output_get_2 "HDRI_Map" (`self.Cubemap`))
      (`MaterialInstanceDynamic.SetTextureParameterValue` _output_get "HDRI_Map" (`self.Cubemap`))
      (`MaterialInstanceDynamic.SetScalarParameterValue` (`self.MaterialInstance`) "LightingDistance" (* (`self.Size`) (`self.LightingDistanceFactor`) 100.0))
      (`MaterialInstanceDynamic.SetScalarParameterValue` (`self.MaterialInstance`) "HDRI_Angle" (* (.yaw (`SceneComponent.K2_GetComponentRotation` (`self.SceneComponent`))) -1.0))
      (`MaterialInstanceDynamic.SetVectorParameterValue` (`self.MaterialInstance`) "ProjectionPosition" (make `LinearColor` (.x (`KismetMathLibrary.GreaterGreater_VectorRotator` (`self.ProjectionCenter`) (`SceneComponent.K2_GetComponentRotation` (`self.SceneComponent`)))) (.y (`KismetMathLibrary.GreaterGreater_VectorRotator` (`self.ProjectionCenter`) (`SceneComponent.K2_GetComponentRotation` (`self.SceneComponent`)))) (.z (`KismetMathLibrary.GreaterGreater_VectorRotator` (`self.ProjectionCenter`) (`SceneComponent.K2_GetComponentRotation` (`self.SceneComponent`))))))
      (`MaterialInstanceDynamic.SetScalarParameterValue` (`self.MaterialInstance`) "Intensity" (`self.Intensity`)))
    (:`then_1`
      (`PrimitiveComponent.SetMaterial` (`self.Geometry`) 0 (`self.MaterialInstance`))
      (`SceneComponent.K2_SetWorldRotation` _scenecomponent (`KismetMathLibrary.MakeRotator` 0.0 0.0 _returnvalue_yaw) false false))))

(fn `UserConstructionScript`
  (`StaticMeshComponent.SetStaticMesh` (`self.Geometry`) (`self.Mesh`))
  (`SceneComponent.SetWorldScale3D` (`self.Geometry`) (`KismetMathLibrary.Conv_DoubleToVector` (/ (`self.Size`) (/ (`.SphereRadius` (`KismetSystemLibrary.GetComponentBounds` (`self.Geometry`))) 50.0))))
  (`self.CreateMaterial`))